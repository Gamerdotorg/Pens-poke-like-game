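; BP_Pokemon_required_past_Point is a world checkpoint that blocks the player until their trainer party contains a Pokémon.
; On overlapping Show_text, it scans the party for any entry with max HP above zero, not current HP.
; If found, it disables Blockign's collision and passes it to the player's VanashingButton; HasPokemon is never reset here.
; Otherwise it keeps collision on and shows the W_Past_point widget until overlap ends.
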(event `self.Show_text.OnComponentBeginOverlap`
  (params (OverlappedComponent :type "PrimitiveComponent Object Reference") (OtherActor :type "Actor Object Reference") (OtherComp :type "PrimitiveComponent Object Reference") (OtherBodyIndex :type Integer) (bFromSweep :type Boolean) (SweepResult :type "HitResult Structure (by ref)"))
  (bind _blockign (`self.Blockign`))
  (bind _asbp_top_down_char (cast `/Game/charecter/BP_top_down_char` OtherActor))
  (set `self.As BP Top Down Char` _asbp_top_down_char)
  (if (== _asbp_top_down_char (`GameplayStatics.GetPlayerCharacter` 0))
    (for _array_element (`.TrainerParty_5_99166060424350E6AB65298B76F38231` (break `/Game/charecter/S_TrainerPokemon` (`/Game/charecter/BP_top_down_char.Trainer Pokemon` (`self.As BP Top Down Char`))))
      (if (not (<= (`.HPMax_15_99BD6E584583F33A1DB10DBF2C4B84CF` (break `/Game/Pokemon/info/S_PokeFinalStats` (`.FinalStats_50_1025B5E14F12CB17F3D943A89782593B` (break `/Game/Pokemon/info/S_PokePartyInfo` _array_element)))) 0.0))
        (set `self.has pokemon?` true)
        (break)))
    (if (`self.has pokemon?`)
      (`PrimitiveComponent.SetCollisionEnabled` _blockign "NoCollision")
      (`/Game/charecter/BP_top_down_char.Vanashing Button` (`self.As BP Top Down Char`) (`self.Blockign`))
      (else
        (bind _returnvalue (`|CreateWidget` "/Game/World/Special_objects/P_R_Past_point/W_Past_point.W_Past_point_C"))
        (`UserWidget.AddToViewport` _returnvalue 0)
        (set `self.Widget ref` _returnvalue)
        (`PrimitiveComponent.SetCollisionEnabled` _blockign "QueryAndPhysics")))))

(event `self.Show_text.OnComponentEndOverlap`
  (params (OverlappedComponent :type "PrimitiveComponent Object Reference") (OtherActor :type "Actor Object Reference") (OtherComp :type "PrimitiveComponent Object Reference") (OtherBodyIndex :type Integer))
  (bind _widget_ref (`self.Widget ref`))
  (bind _asbp_top_down_char (cast `/Game/charecter/BP_top_down_char` OtherActor))
  (if (== _asbp_top_down_char (`GameplayStatics.GetPlayerCharacter` 0))
    (`/Engine/EditorBlueprintResources/StandardMacros.IsValid` _widget_ref
      (:`Is Valid`
        (`Widget.RemoveFromParent` _widget_ref)))))

(fn `UserConstructionScript`)
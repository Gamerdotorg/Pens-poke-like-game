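; Data-driven master NPC for trainers, gym leaders and dialogue characters in a top-down Pokémon-style game.
; BeginPlay loads its DT_NPC_LIst row by name, builds a randomized team, and sizes a facing-based sight box.
; Walking and standing trainers battle on sight; interacting shows dialogue, with gym leaders then starting a badge battle.
; FinalStats runs before each Pokémon's level and base stats update, and rolls IVs separate from those stored.
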(event OnComponentBeginOverlap(SightBox)
  (params (OverlappedComponent :type Primitive%20Component%20Object%20Reference) (OtherActor :type Actor%20Object%20Reference) (OtherComp :type Primitive%20Component%20Object%20Reference) (OtherBodyIndex :type Integer) (bFromSweep :type Boolean) (SweepResult :type Hit%20Result%20Structure%20%28by%20ref%29))
  (bind _asbp_top_down_char (Utilities|Casting|CastToBP_top_down_char OtherActor))
  (Default|SpBattleStart _asbp_top_down_char (Variables|Default|GetTrainer%20Team) false false))

(event OnComponentBeginOverlap(InteractBox)
  (params (OverlappedComponent :type Primitive%20Component%20Object%20Reference) (OtherActor :type Actor%20Object%20Reference) (OtherComp :type Primitive%20Component%20Object%20Reference) (OtherBodyIndex :type Integer) (bFromSweep :type Boolean) (SweepResult :type Hit%20Result%20Structure%20%28by%20ref%29))
  (bind _asbp_top_down_char (Utilities|Casting|CastToBP_top_down_char OtherActor))
  (if (== _asbp_top_down_char (Game|GetPlayerCharacter 0))
    (Input|EnableInput (Game|GetPlayerController 0))))

(event OnComponentEndOverlap(InteractBox)
  (params (OverlappedComponent :type Primitive%20Component%20Object%20Reference) (OtherActor :type Actor%20Object%20Reference) (OtherComp :type Primitive%20Component%20Object%20Reference) (OtherBodyIndex :type Integer))
  (bind _asbp_top_down_char (Utilities|Casting|CastToBP_top_down_char OtherActor))
  (if (== _asbp_top_down_char (Game|GetPlayerCharacter 0))
    (Input|DisableInput (Game|GetPlayerController 0))))

(event Custom|Print%20on%20server
  (params (InString :type String))
  (if (Utilities|Array|IsEmpty InString)
    (Development|PrintString "Empty print")
    (else
      (Development|PrintString InString))))

(event Input|EnhancedActionEvents|EnhancedInputActionIA_Interact
  (params (ActionValue :type Boolean) (ElapsedSeconds :type Float%20%28double-precision%29) (TriggeredSeconds :type Float%20%28double-precision%29) (InputAction :type Input%20Action%20Object%20Reference :default "/Game/charecter/input/IA_Interact.IA_Interact"))
  (switch Utilities|FlowControl|Switch|SwitchonE_NPC_Types (Variables|Default|Get?Type%20is%20this%20NPC)
    (:NewEnumerator0
      (CallFunction|DialogueText :!label _label))
    (:NewEnumerator3
      (goto _label))
    (:NewEnumerator4
      (bind _returnvalue (CallFunction|DialogueText))
      (Utilities|FlowControl|Delay 1.0)
      (Widget|RemovefromParent _returnvalue)
      (CallFunction|GymLeader))
    (:NewEnumerator5
      (goto _label))))

(event EventBeginPlay
  (CallFunction|SetInfo)
  (CallFunction|GivePokemon)
  (switch Utilities|FlowControl|Switch|SwitchonE_Direction_NPC (Variables|Default|GetDirection%20NPC%20is%20Looking)
    (:NewEnumerator4
      (Variables|Default|SetDirectionality "(X=0.000000,Y=-1.000000)")
      (Variables|Default|SetSight%20Box%20Location (+ (Transformation|GetActorLocation self) (* "0.000000,1.000000,0.000000" (* 32.0 (Variables|Default|GetVision%20Distance))) (* (* 18.0 (Variables|Default|GetVision%20Distance)) "0.000000,1.000000,0.000000") "0.000000,-64.000000,0.000000"))
      (Variables|Default|Setsight%20Box%20rotation "0.000000,90.000000,0.000000"))
    (:NewEnumerator0
      (Variables|Default|SetDirectionality "(X=0.000000,Y=1.000000)")
      (Variables|Default|SetSight%20Box%20Location (+ (Transformation|GetActorLocation self) (* "0.000000,-1.000000,0.000000" (* 32.0 (Variables|Default|GetVision%20Distance))) (* "0.000000,-1.000000,0.000000" (* 18.0 (Variables|Default|GetVision%20Distance))) "0.000000,64.000000,0.000000"))
      (Variables|Default|Setsight%20Box%20rotation "0.000000,90.000000,0.000000"))
    (:NewEnumerator1
      (Variables|Default|SetDirectionality "(X=1.000000,Y=0.000000)")
      (Variables|Default|SetSight%20Box%20Location (+ (Transformation|GetActorLocation self) (* "1.000000,0.000000,0.000000" (* 32.0 (Variables|Default|GetVision%20Distance))) (* "1.000000,0.000000,0.000000" (* 18.0 (Variables|Default|GetVision%20Distance))) "-64.000000,0.000000,0.000000"))
      (Variables|Default|Setsight%20Box%20rotation "0, 0, 0"))
    (:NewEnumerator2
      (Variables|Default|SetDirectionality "(X=0.000000,Y=-1.000000)")
      (Variables|Default|SetSight%20Box%20Location (+ (Transformation|GetActorLocation self) (* "0.000000,1.000000,0.000000" (* 32.0 (Variables|Default|GetVision%20Distance))) (* "0.000000,1.000000,0.000000" (* 18.0 (Variables|Default|GetVision%20Distance))) "0.000000,-64.000000,0.000000"))
      (Variables|Default|Setsight%20Box%20rotation "0.000000,90.000000,0.000000"))
    (:NewEnumerator3
      (Variables|Default|SetDirectionality "(X=-1.000000,Y=0.000000)")
      (Variables|Default|SetSight%20Box%20Location (+ (Transformation|GetActorLocation self) (* "-1.000000,0.000000,0.000000" (* 32.0 (Variables|Default|GetVision%20Distance))) (* "-1.000000,0.000000,0.000000" (* 18.0 (Variables|Default|GetVision%20Distance))) "64.000000,0.000000,0.000000"))
      (Variables|Default|Setsight%20Box%20rotation "0, 0, 0")))
  (Rendering|Components|TextRender|SetText (Variables|Default|GetTextRender) (Utilities|Text|ToText(String) (Utilities|String|EnumtoString (Variables|Default|GetDirection%20NPC%20is%20Looking))))
  (Transformation|SetWorldTransform (Variables|Default|GetSight%20Box) (Math|Transform|MakeTransform (Variables|Default|GetSight%20Box%20Location) (Variables|Default|Getsight%20Box%20rotation) (Math|Vector|MakeVector (Variables|Default|GetVision%20Distance) 1.0 1.0)) false true)
  (if (Utilities|Array|IsEmpty (Variables|Default|GetGiven%20Pokemon))
    (Collision|SetCollisionEnabled (Variables|Default|GetSight%20Box) "NoCollision")
    (else
      (switch Utilities|FlowControl|Switch|SwitchonE_NPC_Types (Variables|Default|Get?Type%20is%20this%20NPC)
        (:NewEnumerator0
          (Collision|SetCollisionEnabled (Variables|Default|GetSight%20Box) "NoCollision" :!label _label))
        (:NewEnumerator1
          (Collision|SetCollisionEnabled (Variables|Default|GetSight%20Box) "QueryAndPhysics" :!label _label_2))
        (:NewEnumerator2
          (goto _label_2))
        (:NewEnumerator3
          (goto _label))
        (:NewEnumerator4
          (goto _label))
        (:NewEnumerator5
          (goto _label))
        (:NewEnumerator6
          (goto _label))
        (:NewEnumerator7
          (goto _label))
        (:NewEnumerator8
          (goto _label))))))

(fn ConstructionScript)

(fn DialogueText
  (bind _returnvalue (UserInterface|CreateWidget "/Game/menus/NPC_Talking/Wig_NPC_Dialogue.Wig_NPC_Dialogue_C" 0 (Variables|Dialogue|GetName%20Text) (Variables|Dialogue|GetDialougue%20Text)))
  (UserInterface|Viewport|AddtoViewport _returnvalue 0)
  (return _returnvalue))

(fn GivePokemon
  (for (_array_element _array_index) (Variables|Default|GetGiven%20Pokemon)
    (CallFunction|FinalStats)
    (Variables|Default|SetLevel (.Level (Utilities|Struct|BreakS_Trainer_Party_info _array_element)))
    (bind _returnvalue (Utilities|GetDataTableRow "/Game/Pokemon/info/DT_Pokemon_basic_info.DT_Pokemon_basic_info" (.PokemonName (Utilities|Struct|BreakS_Trainer_Party_info _array_element)))
      (:then
        (Variables|Default|Set%20Base%20Stats (Utilities|Struct|BreakS_PokeBasicInformation _returnvalue))
        (Utilities|Array|SetArrayElem (Variables|Default|GetTrainer%20Team) _array_index (Utilities|Struct|MakeS_PokePartyInfo (.PokemonName (Utilities|Struct|BreakS_Trainer_Party_info _array_element)) (Utilities|String|ToString(Name) (.PokemonName (Utilities|Struct|BreakS_Trainer_Party_info _array_element))) "NewEnumerator0" "None" (.moves (Utilities|Struct|BreakS_Trainer_Party_info _array_element)) 0 1.0 1e+01 (Variables|Default|GetLevel) false "NewEnumerator0" 255 (Variables|Default|Get%20Base%20Stats) (Utilities|Struct|MakeS_PokeIV (Math|Random|RandomIntegerinRange 0 31) (Math|Random|RandomIntegerinRange 0 31) (Math|Random|RandomIntegerinRange 0 31) (Math|Random|RandomIntegerinRange 0 31) (Math|Random|RandomIntegerinRange 0 31) (Math|Random|RandomIntegerinRange 0 31)) (Utilities|Struct|MakeS_PokeEV (Math|Random|RandomIntegerinRange 0 31) (Math|Random|RandomIntegerinRange 0 31) (Math|Random|RandomIntegerinRange 0 31) (Math|Random|RandomIntegerinRange 0 31) (Math|Random|RandomIntegerinRange 0 31) (Math|Random|RandomIntegerinRange 0 31)) (Variables|Default|GetFinal%20Stats_0)))))))

(fn FinalStats
  (bind _returnvalue (Math|Random|RandomIntegerinRange 0 31))
  (bind _returnvalue_2 (Math|Random|RandomIntegerinRange 0 31))
  (bind _returnvalue_3 (Math|Random|RandomIntegerinRange 0 31))
  (bind _returnvalue_4 (Math|Random|RandomIntegerinRange 0 31))
  (bind _returnvalue_5 (Math|Random|RandomIntegerinRange 0 31))
  (bind _returnvalue_6 (Math|Random|RandomIntegerinRange 0 31))
  (bind _level (Variables|Default|GetLevel))
  (bind __base_stats (Variables|Default|Get%20Base%20Stats))
  (bind (_hp _attack _defence _spattack _spdefence _speed _acuracy _evasive) (Utilities|Struct|BreakS_PokeBaseStats __base_stats))
  (bind _s_pokeiv (Utilities|Struct|MakeS_PokeIV _returnvalue_2 _returnvalue_3 _returnvalue_4 _returnvalue_5 _returnvalue_6 _returnvalue))
  (bind (_hp_2 _attk _def _sp_attk _sp_def _speed_2) (Utilities|Struct|BreakS_PokeIV _s_pokeiv))
  (bind _returnvalue_7 (|((((((HPBS*2)+HP)+CL)/100)+CL)+10) _hp _hp_2 _level))
  (bind _returnvalue_8 (|((((((StatBS*2)+IV)*CL)/100)+CL)+5) _speed _speed_2 _level))
  (bind _returnvalue_9 (|((((((StatBS*2)+IV)*CL)/100)+CL)+5) _attack _attk _level))
  (bind _returnvalue_10 (|((((((StatBS*2)+IV)*CL)/100)+CL)+5) _defence _def _level))
  (bind _returnvalue_11 (|((((((StatBS*2)+IV)*CL)/100)+CL)+5) _spattack _sp_attk _level))
  (bind _returnvalue_12 (|((((((StatBS*2)+IV)*CL)/100)+CL)+5) _spdefence _sp_def _level))
  (bind _returnvalue_13 (Math|Float|Round _returnvalue_8))
  (bind _returnvalue_14 (Math|Float|Round _returnvalue_7))
  (bind _returnvalue_15 (Math|Float|Round _returnvalue_9))
  (bind _returnvalue_16 (Math|Float|Round _returnvalue_10))
  (bind _returnvalue_17 (Math|Float|Round _returnvalue_11))
  (bind _returnvalue_18 (Math|Float|Round _returnvalue_12))
  (bind _returnvalue_19 (Math|Conversions|ToFloat(Integer) _returnvalue_14))
  (bind _returnvalue_20 (Math|Conversions|ToFloat(Integer) _returnvalue_13))
  (bind _returnvalue_21 (Math|Conversions|ToFloat(Integer) _returnvalue_15))
  (bind _returnvalue_22 (Math|Conversions|ToFloat(Integer) _returnvalue_16))
  (bind _returnvalue_23 (Math|Conversions|ToFloat(Integer) _returnvalue_17))
  (bind _returnvalue_24 (Math|Conversions|ToFloat(Integer) _returnvalue_18))
  (Variables|Default|SetFinal%20Stats_0 (Utilities|Struct|MakeS_PokeFinalStats _returnvalue_19 _returnvalue_19 _returnvalue_21 _returnvalue_21 _returnvalue_22 _returnvalue_22 _returnvalue_23 _returnvalue_23 _returnvalue_24 _returnvalue_24 _returnvalue_20 _returnvalue_20 _evasive _evasive _acuracy _acuracy))
  (return))

(fn SetInfo
  (bind _returnvalue (Utilities|GetDataTableRow "/Game/PokeTrainer/npc_Master/DT_NPC_LIst.DT_NPC_LIst" (Utilities|String|StringToName (Utilities|String|Replace (Utilities|String|ToString(Text) (Variables|Dialogue|GetName%20Text)) " " "_")))
    (:then
      (Variables|Dialogue|SetDialougue%20Text (.NPCDialogue (Utilities|Struct|BreakS_NPC_List _returnvalue)))
      (Variables|Default|Set?Type%20is%20this%20NPC (.NPCType (Utilities|Struct|BreakS_NPC_List _returnvalue)))
      (Variables|Default|SetGiven%20Pokemon (.GivenPokemon (Utilities|Struct|BreakS_NPC_List _returnvalue)))
      (Variables|Default|SetVision%20Distance (.VisionDistance (Utilities|Struct|BreakS_NPC_List _returnvalue)))
      (Class|PaperZDAnimationComponent|SetAnimInstanceClass (Variables|Default|GetPaperZDAnimation) (.Animationclass (Utilities|Struct|BreakS_NPC_List _returnvalue)))
      (Variables|Default|SetGym%20Badge (.GymBadge (Utilities|Struct|BreakS_NPC_List _returnvalue))))
    (:RowNotFound
      (Development|PrintString "Hello"))))

(fn GymLeader
  (bind _asbp_top_down_char (Utilities|Casting|CastToBP_top_down_char (Game|GetPlayerCharacter 0)))
  (Default|SpBattleStart _asbp_top_down_char (Variables|Default|GetTrainer%20Team) false true (Variables|Default|GetGym%20Badge)))
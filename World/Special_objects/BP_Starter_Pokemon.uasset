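; Interactable starter Pokémon that offers itself to a player whose party is still empty.
; Its overlap box toggles input for the player character, so interact works only up close.
; The first interact rolls shininess one time and writes level 5, shiny and gender into the starter data; the gender roll can only yield one value.
; With no party Pokémon found, it opens the accept widget in UI-only input mode.
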(event `Roll For Info`
  ;[1 1 1] set info
  (`/Engine/EditorBlueprintResources/StandardMacros.DoOnce` false
    (:`Completed`
      (if (== (`KismetMathLibrary.RandomIntegerInRange` 1 (`self.Shiny rate`)) 1)
        (set `self.isShiny` true)
        (else
          (set `self.isShiny` false)))
      (if (>= (`KismetMathLibrary.RandomIntegerInRange` 1 50) 51)
        (set `self.Gender` "NewEnumerator2")
        (else
          (set `self.Gender` "NewEnumerator1")))
      (bind _structout (setmembers `/Game/Pokemon/info/S_PokePartyInfo` :`StructRef` (`self.Starter Pokemon`) :`Current Level` 5 :`Shiny` (`self.isShiny`) :`Gender` (`self.Gender`)))
      (set `self.Starter Pokemon` _structout))))

(event `self.Box.OnComponentBeginOverlap`
  (params (OverlappedComponent :type "PrimitiveComponent Object Reference") (OtherActor :type "Actor Object Reference") (OtherComp :type "PrimitiveComponent Object Reference") (OtherBodyIndex :type Integer) (bFromSweep :type Boolean) (SweepResult :type "HitResult Structure (by ref)"))
  ;[1 1 1] Set Overlap
  (bind _asbp_top_down_char (cast `/Game/charecter/BP_top_down_char` OtherActor))
  (bind _output_get (set `self.As BP Top Down Char` _asbp_top_down_char))
  (if (== _output_get (`GameplayStatics.GetPlayerCharacter` 0))
    (`self.EnableInput` (`GameplayStatics.GetPlayerController` 0))))

(event `self.Box.OnComponentEndOverlap`
  (params (OverlappedComponent :type "PrimitiveComponent Object Reference") (OtherActor :type "Actor Object Reference") (OtherComp :type "PrimitiveComponent Object Reference") (OtherBodyIndex :type Integer))
  ;[1 1 1] Set Overlap
  (bind _asbp_top_down_char (cast `/Game/charecter/BP_top_down_char` OtherActor))
  (if (== (`GameplayStatics.GetPlayerCharacter` 0) _asbp_top_down_char)
    (`self.DisableInput` (`GameplayStatics.GetPlayerController` 0))))

(event `EnhancedInput|/Game/charecter/input/IA_Interact`
  (params (ActionValue :type Boolean) (ElapsedSeconds :type "Float (double-precision)") (TriggeredSeconds :type "Float (double-precision)") (InputAction :type "InputAction Object Reference" :default "/Game/charecter/input/IA_Interact.IA_Interact"))
  (bind _returnvalue (`GameplayStatics.GetPlayerController` 0))
  ;[1 1 1] interact with starter
  (:`Triggered`
    (`self.Roll For Info`)
    (for _array_element (`.TrainerParty_5_99166060424350E6AB65298B76F38231` (break `/Game/charecter/S_TrainerPokemon` (`/Game/charecter/BP_top_down_char.Trainer Pokemon` (`self.As BP Top Down Char`))))
      (if (not (== (`.PokemonName_25_B21F389046EE06E05ABE5486275EE353` (break `/Game/Pokemon/info/S_PokePartyInfo` _array_element)) "None"))
        (set `self.hasPokemon` true)
        (break)))
    (if (not (`self.hasPokemon`))
      (set `PlayerController.bShowMouseCursor` true _returnvalue)
      (`WidgetBlueprintLibrary.SetInputMode_UIOnlyEx` _returnvalue null)
      (bind _returnvalue_2 (`|CreateWidget` "/Game/Pokemon/info/Pokemon_Starter/Accept_pokemon_widget.Accept_pokemon_widget_C" null (`self.pokemonName`) (`self.Starter Pokemon`) (`self.PokeBall`)))
      (`UserWidget.AddToViewport` _returnvalue_2 0))))

(fn `UserConstructionScript`)
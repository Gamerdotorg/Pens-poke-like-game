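; Data-driven Pokémon NPC in testing, covering trainers, gym leaders, special Pokémon, healers and dialogue characters.
; On BeginPlay it loads its data-table row, builds a team with random IVs/EVs, and sizes a facing-aligned sight box.
; Unbeaten trainers start a test battle on sight.
; Interacting shows timed dialogue, then may start gym battles (rematches at 1.5x level) or special encounters, or heal the party and set respawn.
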(event OnComponentBeginOverlap(SightBox)
  (params (OverlappedComponent :type Primitive%20Component%20Object%20Reference) (OtherActor :type Actor%20Object%20Reference) (OtherComp :type Primitive%20Component%20Object%20Reference) (OtherBodyIndex :type Integer) (bFromSweep :type Boolean) (SweepResult :type Hit%20Result%20Structure%20%28by%20ref%29))
  (bind _returnvalue (Game|GetPlayerCharacter 0))
  (bind _asbp_top_down_char (Utilities|Casting|CastToBP_top_down_char OtherActor))
  (if (== _asbp_top_down_char _returnvalue)
    (bind _asbp_top_down_char_2 (Utilities|Casting|CastToBP_top_down_char _returnvalue))
    (Variables|Default|SetTrainer%20been%20beaten? false)
    (bind _array_element (Utilities|Array|ForEachLoopwithBreak (Variables|/Game/charecter/BP_top_down_char.BP_top_down_char_C|GetNPC%20Beaten _asbp_top_down_char_2) :!label _label)
      (:LoopBody
        (if (== _array_element (Utilities|Struct|BreakDataTableRowHandle (Variables|Info|GetTrainer%20Data%20Table)))
          (Variables|Default|SetTrainer%20been%20beaten? true)
          (goto _label Break)))
      (:Completed
        (if (not (Variables|Default|GetTrainer%20been%20beaten?))
          (Default|TestingBattleStart _asbp_top_down_char_2))))))

(event OnComponentBeginOverlap(InteractBox)
  (params (OverlappedComponent :type Primitive%20Component%20Object%20Reference) (OtherActor :type Actor%20Object%20Reference) (OtherComp :type Primitive%20Component%20Object%20Reference) (OtherBodyIndex :type Integer) (bFromSweep :type Boolean) (SweepResult :type Hit%20Result%20Structure%20%28by%20ref%29))
  (bind _asbp_top_down_char (Utilities|Casting|CastToBP_top_down_char OtherActor))
  (if (== _asbp_top_down_char (Game|GetPlayerCharacter 0))
    (Input|EnableInput (Game|GetPlayerController 0))))

(event OnComponentEndOverlap(InteractBox)
  (params (OverlappedComponent :type Primitive%20Component%20Object%20Reference) (OtherActor :type Actor%20Object%20Reference) (OtherComp :type Primitive%20Component%20Object%20Reference) (OtherBodyIndex :type Integer))
  (bind _asbp_top_down_char (Utilities|Casting|CastToBP_top_down_char OtherActor))
  (if (== _asbp_top_down_char (Game|GetPlayerCharacter 0))
    (Input|DisableInput (Game|GetPlayerController 0))))

(event Input|EnhancedActionEvents|EnhancedInputActionIA_Interact
  (params (ActionValue :type Boolean) (ElapsedSeconds :type Float%20%28double-precision%29) (TriggeredSeconds :type Float%20%28double-precision%29) (InputAction :type Input%20Action%20Object%20Reference :default "/Game/charecter/input/IA_Interact.IA_Interact"))
  (switch Utilities|FlowControl|Switch|SwitchonE_NPC_Types (Variables|Default|Get?Type%20is%20this%20NPC)
    (:NewEnumerator0
      (bind _returnvalue (CallFunction|DialogueText :!label _label))
      (Utilities|FlowControl|Delay 1.0)
      (Widget|RemovefromParent _returnvalue))
    (:NewEnumerator1
      (goto _label))
    (:NewEnumerator2
      (goto _label))
    (:NewEnumerator3
      (goto _label))
    (:NewEnumerator4
      (bind _returnvalue_2 (CallFunction|DialogueText))
      (Utilities|FlowControl|Delay 1.0)
      (Widget|RemovefromParent _returnvalue_2)
      (CallFunction|GymLeader))
    (:NewEnumerator5
      (goto _label))
    (:NewEnumerator7
      (bind _returnvalue_3 (CallFunction|DialogueText))
      (Utilities|FlowControl|Delay 1.0)
      (Widget|RemovefromParent _returnvalue_3)
      (CallFunction|SpecialPokemon))
    (:NewEnumerator9
      (bind _returnvalue_4 (CallFunction|DialogueText))
      (Utilities|FlowControl|Delay 1.0)
      (CallFunction|HealPokemon)
      (Widget|RemovefromParent _returnvalue_4))))

(event EventBeginPlay
  (CallFunction|SetInfo)
  (CallFunction|GivePokemon)
  (switch Utilities|FlowControl|Switch|SwitchonE_Direction_NPC (Variables|Info|GetDirection%20NPC%20is%20Looking)
    (:NewEnumerator4
      (Variables|Default|SetSight%20Box%20Location (+ (Transformation|GetActorLocation self) (* "0.000000,1.000000,0.000000" (* 32.0 (Variables|Default|GetVision%20Distance))) (* (* 18.0 (Variables|Default|GetVision%20Distance)) "0.000000,1.000000,0.000000") "0.000000,-64.000000,0.000000"))
      (Variables|Default|Setsight%20Box%20rotation "0.000000,90.000000,0.000000"))
    (:NewEnumerator0
      (Variables|Default|SetSight%20Box%20Location (+ (Transformation|GetActorLocation self) (* "0.000000,-1.000000,0.000000" (* 32.0 (Variables|Default|GetVision%20Distance))) (* "0.000000,-1.000000,0.000000" (* 18.0 (Variables|Default|GetVision%20Distance))) "0.000000,64.000000,0.000000"))
      (Variables|Default|Setsight%20Box%20rotation "0.000000,90.000000,0.000000"))
    (:NewEnumerator1
      (Variables|Default|SetSight%20Box%20Location (+ (Transformation|GetActorLocation self) (* "1.000000,0.000000,0.000000" (* 32.0 (Variables|Default|GetVision%20Distance))) (* "1.000000,0.000000,0.000000" (* 18.0 (Variables|Default|GetVision%20Distance))) "-64.000000,0.000000,0.000000"))
      (Variables|Default|Setsight%20Box%20rotation "0, 0, 0"))
    (:NewEnumerator2
      (Variables|Default|SetSight%20Box%20Location (+ (Transformation|GetActorLocation self) (* "0.000000,1.000000,0.000000" (* 32.0 (Variables|Default|GetVision%20Distance))) (* "0.000000,1.000000,0.000000" (* 18.0 (Variables|Default|GetVision%20Distance))) "0.000000,-64.000000,0.000000"))
      (Variables|Default|Setsight%20Box%20rotation "0.000000,90.000000,0.000000"))
    (:NewEnumerator3
      (Variables|Default|SetSight%20Box%20Location (+ (Transformation|GetActorLocation self) (* "-1.000000,0.000000,0.000000" (* 32.0 (Variables|Default|GetVision%20Distance))) (* "-1.000000,0.000000,0.000000" (* 18.0 (Variables|Default|GetVision%20Distance))) "64.000000,0.000000,0.000000"))
      (Variables|Default|Setsight%20Box%20rotation "0, 0, 0")))
  (Transformation|SetWorldTransform (Variables|Default|GetSight%20Box) (Math|Transform|MakeTransform (Variables|Default|GetSight%20Box%20Location) (Variables|Default|Getsight%20Box%20rotation) (Math|Vector|MakeVector (Variables|Default|GetVision%20Distance) 1.0 1.0)) false true)
  (if (Utilities|Array|IsEmpty (Variables|Default|GetGiven%20Pokemon))
    (Collision|SetCollisionEnabled (Variables|Default|GetSight%20Box) "NoCollision")
    (else
      (switch Utilities|FlowControl|Switch|SwitchonE_NPC_Types (Variables|Default|Get?Type%20is%20this%20NPC)
        (:NewEnumerator0
          (Collision|SetCollisionEnabled (Variables|Default|GetSight%20Box) "NoCollision" :!label _label))
        (:NewEnumerator1
          (Collision|SetCollisionEnabled (Variables|Default|GetSight%20Box) "QueryAndPhysics" :!label _label_2))
        (:NewEnumerator2
          (goto _label_2))
        (:NewEnumerator3
          (goto _label))
        (:NewEnumerator4
          (goto _label))
        (:NewEnumerator5
          (goto _label))
        (:NewEnumerator6
          (goto _label))
        (:NewEnumerator7
          (goto _label))
        (:NewEnumerator8
          (goto _label))
        (:NewEnumerator9
          (goto _label))))))

(fn ConstructionScript)

(fn DialogueText
  (bind _returnvalue (UserInterface|CreateWidget "/Game/menus/NPC_Talking/Wig_NPC_Dialogue.Wig_NPC_Dialogue_C" 0 (Utilities|Text|ToText(Name) (Variables|Default|GetTrainer%20Name)) (Variables|Dialogue|GetDialougue%20Text)))
  (UserInterface|Viewport|AddtoViewport _returnvalue 0)
  (return _returnvalue))

(fn GivePokemon
  (for (_array_element _array_index) (Variables|Default|GetGiven%20Pokemon)
    (Variables|Default|SetLevel (.Level (Utilities|Struct|BreakS_Trainer_Party_info _array_element)))
    (bind _returnvalue (Utilities|GetDataTableRow "/Game/Pokemon/info/DT_Pokemon_basic_info.DT_Pokemon_basic_info" (.PokemonName (Utilities|Struct|BreakS_Trainer_Party_info _array_element)))
      (:then
        (Variables|Default|Set%20Base%20Stats (Utilities|Struct|BreakS_PokeBasicInformation _returnvalue))
        (CallFunction|FinalStats)
        (Utilities|Array|SetArrayElem (Variables|Default|GetTrainer%20Team) _array_index (Utilities|Struct|MakeS_PokePartyInfo (.PokemonName (Utilities|Struct|BreakS_Trainer_Party_info _array_element)) (Utilities|String|ToString(Name) (.PokemonName (Utilities|Struct|BreakS_Trainer_Party_info _array_element))) "NewEnumerator0" "None" (.moves (Utilities|Struct|BreakS_Trainer_Party_info _array_element)) 0 1.0 1e+01 (Variables|Default|GetLevel) false "NewEnumerator0" 255 (Variables|Default|Get%20Base%20Stats) (Utilities|Struct|MakeS_PokeIV (Math|Random|RandomIntegerinRange 0 31) (Math|Random|RandomIntegerinRange 0 31) (Math|Random|RandomIntegerinRange 0 31) (Math|Random|RandomIntegerinRange 0 31) (Math|Random|RandomIntegerinRange 0 31) (Math|Random|RandomIntegerinRange 0 31)) (Utilities|Struct|MakeS_PokeEV (Math|Random|RandomIntegerinRange 0 31) (Math|Random|RandomIntegerinRange 0 31) (Math|Random|RandomIntegerinRange 0 31) (Math|Random|RandomIntegerinRange 0 31) (Math|Random|RandomIntegerinRange 0 31) (Math|Random|RandomIntegerinRange 0 31)) (Variables|Default|GetFinal%20Stats_0)))))))

(fn FinalStats
  (bind _returnvalue (Math|Random|RandomIntegerinRange 0 31))
  (bind _returnvalue_2 (Math|Random|RandomIntegerinRange 0 31))
  (bind _returnvalue_3 (Math|Random|RandomIntegerinRange 0 31))
  (bind _returnvalue_4 (Math|Random|RandomIntegerinRange 0 31))
  (bind _returnvalue_5 (Math|Random|RandomIntegerinRange 0 31))
  (bind _returnvalue_6 (Math|Random|RandomIntegerinRange 0 31))
  (bind _level (Variables|Default|GetLevel))
  (bind __base_stats (Variables|Default|Get%20Base%20Stats))
  (bind (_hp _attack _defence _spattack _spdefence _speed _acuracy _evasive) (Utilities|Struct|BreakS_PokeBaseStats __base_stats))
  (bind _s_pokeiv (Utilities|Struct|MakeS_PokeIV _returnvalue_2 _returnvalue_3 _returnvalue_4 _returnvalue_5 _returnvalue_6 _returnvalue))
  (bind (_hp_2 _attk _def _sp_attk _sp_def _speed_2) (Utilities|Struct|BreakS_PokeIV _s_pokeiv))
  (bind _returnvalue_7 (|((((((HPBS*2)+HP)+CL)/100)+CL)+10) _hp _hp_2 _level))
  (bind _returnvalue_8 (|((((((StatBS*2)+IV)*CL)/100)+CL)+5) _speed _speed_2 _level))
  (bind _returnvalue_9 (|((((((StatBS*2)+IV)*CL)/100)+CL)+5) _attack _attk _level))
  (bind _returnvalue_10 (|((((((StatBS*2)+IV)*CL)/100)+CL)+5) _defence _def _level))
  (bind _returnvalue_11 (|((((((StatBS*2)+IV)*CL)/100)+CL)+5) _spattack _sp_attk _level))
  (bind _returnvalue_12 (|((((((StatBS*2)+IV)*CL)/100)+CL)+5) _spdefence _sp_def _level))
  (bind _returnvalue_13 (Math|Float|Round _returnvalue_8))
  (bind _returnvalue_14 (Math|Float|Round _returnvalue_7))
  (bind _returnvalue_15 (Math|Float|Round _returnvalue_9))
  (bind _returnvalue_16 (Math|Float|Round _returnvalue_10))
  (bind _returnvalue_17 (Math|Float|Round _returnvalue_11))
  (bind _returnvalue_18 (Math|Float|Round _returnvalue_12))
  (bind _returnvalue_19 (Math|Conversions|ToFloat(Integer) _returnvalue_14))
  (bind _returnvalue_20 (Math|Conversions|ToFloat(Integer) _returnvalue_13))
  (bind _returnvalue_21 (Math|Conversions|ToFloat(Integer) _returnvalue_15))
  (bind _returnvalue_22 (Math|Conversions|ToFloat(Integer) _returnvalue_16))
  (bind _returnvalue_23 (Math|Conversions|ToFloat(Integer) _returnvalue_17))
  (bind _returnvalue_24 (Math|Conversions|ToFloat(Integer) _returnvalue_18))
  (Variables|Default|SetFinal%20Stats_0 (Utilities|Struct|MakeS_PokeFinalStats _returnvalue_19 _returnvalue_19 _returnvalue_21 _returnvalue_21 _returnvalue_22 _returnvalue_22 _returnvalue_23 _returnvalue_23 _returnvalue_24 _returnvalue_24 _returnvalue_20 _returnvalue_20 _evasive _evasive _acuracy _acuracy))
  (return))

(fn SetInfo
  (bind _returnvalue (Utilities|GetDataTableRow "/Game/Testing/npc_Master/DT_NPC_LIst.DT_NPC_LIst" (Utilities|Struct|BreakDataTableRowHandle (Variables|Info|GetTrainer%20Data%20Table)))
    (:then
      (Variables|Dialogue|SetDialougue%20Text (.NPCDialogue (Utilities|Struct|BreakS_NPC_List _returnvalue)))
      (Variables|Default|Set?Type%20is%20this%20NPC (.NPCType (Utilities|Struct|BreakS_NPC_List _returnvalue)))
      (Variables|Default|SetGiven%20Pokemon (.GivenPokemon (Utilities|Struct|BreakS_NPC_List _returnvalue)))
      (Variables|Default|SetVision%20Distance (.VisionDistance (Utilities|Struct|BreakS_NPC_List _returnvalue)))
      (Variables|Default|SetGym%20Badge (.GymBadge (Utilities|Struct|BreakS_NPC_List _returnvalue)))
      (bind _returnvalue_2 (Utilities|GetDataTableRow "/Game/Testing/npc_Master/DT_NPC_LIst.DT_NPC_LIst" (Utilities|Struct|BreakDataTableRowHandle (Variables|Info|GetTrainer%20Data%20Table)))
        (:then
          (Variables|Default|SetTrainer%20Name (Utilities|String|StringToName (Utilities|String|ToString(Text) (Utilities|Struct|BreakS_NPC_List _returnvalue_2)))))))))

(fn GymLeader
  (bind _asbp_top_down_char (Utilities|Casting|CastToBP_top_down_char (Game|GetPlayerCharacter 0)))
  (Variables|Default|SetTrainer%20been%20beaten? false)
  (bind _array_element (Utilities|Array|ForEachLoopwithBreak (Variables|/Game/charecter/BP_top_down_char.BP_top_down_char_C|GetGym%20Badges _asbp_top_down_char) :!label _label)
    (:LoopBody
      (if (Utilities|Enum|Equal(Enum) _array_element (Variables|Default|GetGym%20Badge))
        (Variables|Default|SetTrainer%20been%20beaten? true)
        (goto _label Break)))
    (:Completed
      (if (Variables|Default|GetTrainer%20been%20beaten?)
        (for (_array_element_2 _array_index) (Variables|Default|GetTrainer%20Team)
          (bind _s_pokefinalstats (CallFunction|FinalStatsBeatenGymLeader))
          (Utilities|Array|SetArrayElem (Variables|Default|GetGym%20Beaten%20Team) _array_index (Utilities|Struct|MakeS_PokePartyInfo (.PokemonName (Utilities|Struct|BreakS_PokePartyInfo _array_element_2)) (.PokeGivenName (Utilities|Struct|BreakS_PokePartyInfo _array_element_2)) "NewEnumerator0" (.ItemHeld (Utilities|Struct|BreakS_PokePartyInfo _array_element_2)) (.MoveSlots (Utilities|Struct|BreakS_PokePartyInfo _array_element_2)) (.LearnedMoves (Utilities|Struct|BreakS_PokePartyInfo _array_element_2)) (.CurrentXP (Utilities|Struct|BreakS_PokePartyInfo _array_element_2)) (.MaxXP (Utilities|Struct|BreakS_PokePartyInfo _array_element_2)) (+ (.CurrentLevel (Utilities|Struct|BreakS_PokePartyInfo _array_element_2)) (/ (.CurrentLevel (Utilities|Struct|BreakS_PokePartyInfo _array_element_2)) 2)) (.Shiny (Utilities|Struct|BreakS_PokePartyInfo _array_element_2)) (.Gender (Utilities|Struct|BreakS_PokePartyInfo _array_element_2)) (.Hapiness (Utilities|Struct|BreakS_PokePartyInfo _array_element_2)) (.Basestats (Utilities|Struct|BreakS_PokePartyInfo _array_element_2)) (.PokeIvs (Utilities|Struct|BreakS_PokePartyInfo _array_element_2)) (.PokeEVs (Utilities|Struct|BreakS_PokePartyInfo _array_element_2)) _s_pokefinalstats)))
        (Default|SpBattleStart _asbp_top_down_char (Variables|Default|GetGym%20Beaten%20Team) false true (Variables|Default|GetGym%20Badge) (Utilities|Struct|BreakDataTableRowHandle (Variables|Info|GetTrainer%20Data%20Table)))
        (else
          (Default|SpBattleStart _asbp_top_down_char (Variables|Default|GetTrainer%20Team) false true (Variables|Default|GetGym%20Badge) (Utilities|Struct|BreakDataTableRowHandle (Variables|Info|GetTrainer%20Data%20Table))))))))

(fn HealPokemon
  (bind _asbp_top_down_char (Utilities|Casting|CastToBP_top_down_char (Game|GetPlayerCharacter 0)))
  (for (_array_element _array_index) (.TrainerParty (Utilities|Struct|BreakS_TrainerPokemon (Variables|/Game/charecter/BP_top_down_char.BP_top_down_char_C|GetTrainer%20Pokemon _asbp_top_down_char)))
    (Utilities|Array|SetArrayElem (.TrainerParty (Utilities|Struct|BreakS_TrainerPokemon (Variables|/Game/charecter/BP_top_down_char.BP_top_down_char_C|GetTrainer%20Pokemon _asbp_top_down_char))) _array_index (Utilities|Struct|MakeS_PokePartyInfo (.PokemonName (Utilities|Struct|BreakS_PokePartyInfo _array_element)) (.PokeGivenName (Utilities|Struct|BreakS_PokePartyInfo _array_element)) "NewEnumerator0" (.ItemHeld (Utilities|Struct|BreakS_PokePartyInfo _array_element)) (.MoveSlots (Utilities|Struct|BreakS_PokePartyInfo _array_element)) (.LearnedMoves (Utilities|Struct|BreakS_PokePartyInfo _array_element)) (.CurrentXP (Utilities|Struct|BreakS_PokePartyInfo _array_element)) (.MaxXP (Utilities|Struct|BreakS_PokePartyInfo _array_element)) (.CurrentLevel (Utilities|Struct|BreakS_PokePartyInfo _array_element)) (.Shiny (Utilities|Struct|BreakS_PokePartyInfo _array_element)) (.Gender (Utilities|Struct|BreakS_PokePartyInfo _array_element)) (.Hapiness (Utilities|Struct|BreakS_PokePartyInfo _array_element)) (.Basestats (Utilities|Struct|BreakS_PokePartyInfo _array_element)) (.PokeIvs (Utilities|Struct|BreakS_PokePartyInfo _array_element)) (.PokeEVs (Utilities|Struct|BreakS_PokePartyInfo _array_element)) (Utilities|Struct|MakeS_PokeFinalStats (.HPMax (Utilities|Struct|BreakS_PokeFinalStats (.FinalStats (Utilities|Struct|BreakS_PokePartyInfo _array_element)))) (.HPMax (Utilities|Struct|BreakS_PokeFinalStats (.FinalStats (Utilities|Struct|BreakS_PokePartyInfo _array_element)))) (.ATTKMax (Utilities|Struct|BreakS_PokeFinalStats (.FinalStats (Utilities|Struct|BreakS_PokePartyInfo _array_element)))) (.ATTKMax (Utilities|Struct|BreakS_PokeFinalStats (.FinalStats (Utilities|Struct|BreakS_PokePartyInfo _array_element)))) (.DEFMax (Utilities|Struct|BreakS_PokeFinalStats (.FinalStats (Utilities|Struct|BreakS_PokePartyInfo _array_element)))) (.DEFMax (Utilities|Struct|BreakS_PokeFinalStats (.FinalStats (Utilities|Struct|BreakS_PokePartyInfo _array_element)))) (.SPATTKMax (Utilities|Struct|BreakS_PokeFinalStats (.FinalStats (Utilities|Struct|BreakS_PokePartyInfo _array_element)))) (.SPATTKMax (Utilities|Struct|BreakS_PokeFinalStats (.FinalStats (Utilities|Struct|BreakS_PokePartyInfo _array_element)))) (.SPDEFMax (Utilities|Struct|BreakS_PokeFinalStats (.FinalStats (Utilities|Struct|BreakS_PokePartyInfo _array_element)))) (.SPDEFMax (Utilities|Struct|BreakS_PokeFinalStats (.FinalStats (Utilities|Struct|BreakS_PokePartyInfo _array_element)))) (.SpeedMax (Utilities|Struct|BreakS_PokeFinalStats (.FinalStats (Utilities|Struct|BreakS_PokePartyInfo _array_element)))) (.SpeedMax (Utilities|Struct|BreakS_PokeFinalStats (.FinalStats (Utilities|Struct|BreakS_PokePartyInfo _array_element)))) (.EvasivenessMax (Utilities|Struct|BreakS_PokeFinalStats (.FinalStats (Utilities|Struct|BreakS_PokePartyInfo _array_element)))) (.EvasivenessMax (Utilities|Struct|BreakS_PokeFinalStats (.FinalStats (Utilities|Struct|BreakS_PokePartyInfo _array_element)))) (.AcuracyMax (Utilities|Struct|BreakS_PokeFinalStats (.FinalStats (Utilities|Struct|BreakS_PokePartyInfo _array_element)))) (.AcuracyMax (Utilities|Struct|BreakS_PokeFinalStats (.FinalStats (Utilities|Struct|BreakS_PokePartyInfo _array_element)))))))
    (bind _asbp_top_down_char_2 (Utilities|Casting|CastToBP_top_down_char (Game|GetPlayerCharacter 0)))
    (Default|FuncSetRespawnLoaction _asbp_top_down_char_2 (Transformation|GetActorLocation _asbp_top_down_char_2))))

(fn SpecialPokemon
  (bind _asbp_top_down_char (Utilities|Casting|CastToBP_top_down_char (Game|GetPlayerCharacter 0)))
  (Variables|Default|SetTrainer%20been%20beaten? false)
  (bind _array_element (Utilities|Array|ForEachLoopwithBreak (Variables|/Game/charecter/BP_top_down_char.BP_top_down_char_C|GetNPC%20Beaten _asbp_top_down_char) :!label _label)
    (:LoopBody
      (if (== _array_element (Utilities|Struct|BreakDataTableRowHandle (Variables|Info|GetTrainer%20Data%20Table)))
        (Variables|Default|SetTrainer%20been%20beaten? true)
        (goto _label Break)))
    (:Completed
      (if (not (Variables|Default|GetTrainer%20been%20beaten?))
        (Default|SpBattleStart _asbp_top_down_char (Variables|Default|GetTrainer%20Team) true false (Variables|Default|GetGym%20Badge) (Utilities|Struct|BreakDataTableRowHandle (Variables|Info|GetTrainer%20Data%20Table)))))))

(fn FinalStatsBeatenGymLeader
  (bind _returnvalue (Math|Random|RandomIntegerinRange 0 31))
  (bind _returnvalue_2 (Math|Random|RandomIntegerinRange 0 31))
  (bind _returnvalue_3 (Math|Random|RandomIntegerinRange 0 31))
  (bind _returnvalue_4 (Math|Random|RandomIntegerinRange 0 31))
  (bind _returnvalue_5 (Math|Random|RandomIntegerinRange 0 31))
  (bind _returnvalue_6 (Math|Random|RandomIntegerinRange 0 31))
  (bind _level (Variables|Default|GetLevel))
  (bind __base_stats (Variables|Default|Get%20Base%20Stats))
  (bind (_hp _attack _defence _spattack _spdefence _speed _acuracy _evasive) (Utilities|Struct|BreakS_PokeBaseStats __base_stats))
  (bind _s_pokeiv (Utilities|Struct|MakeS_PokeIV _returnvalue_2 _returnvalue_3 _returnvalue_4 _returnvalue_5 _returnvalue_6 _returnvalue))
  (bind _returnvalue_7 (/ _level 2))
  (bind (_hp_2 _attk _def _sp_attk _sp_def _speed_2) (Utilities|Struct|BreakS_PokeIV _s_pokeiv))
  (bind _returnvalue_8 (+ _level _returnvalue_7))
  (bind _returnvalue_9 (|((((((HPBS*2)+HP)+CL)/100)+CL)+10) _hp _hp_2 _returnvalue_8))
  (bind _returnvalue_10 (|((((((StatBS*2)+IV)*CL)/100)+CL)+5) _speed _speed_2 _returnvalue_8))
  (bind _returnvalue_11 (|((((((StatBS*2)+IV)*CL)/100)+CL)+5) _attack _attk _returnvalue_8))
  (bind _returnvalue_12 (|((((((StatBS*2)+IV)*CL)/100)+CL)+5) _defence _def _returnvalue_8))
  (bind _returnvalue_13 (|((((((StatBS*2)+IV)*CL)/100)+CL)+5) _spattack _sp_attk _returnvalue_8))
  (bind _returnvalue_14 (|((((((StatBS*2)+IV)*CL)/100)+CL)+5) _spdefence _sp_def _returnvalue_8))
  (bind _returnvalue_15 (Math|Float|Round _returnvalue_10))
  (bind _returnvalue_16 (Math|Float|Round _returnvalue_9))
  (bind _returnvalue_17 (Math|Float|Round _returnvalue_11))
  (bind _returnvalue_18 (Math|Float|Round _returnvalue_12))
  (bind _returnvalue_19 (Math|Float|Round _returnvalue_13))
  (bind _returnvalue_20 (Math|Float|Round _returnvalue_14))
  (bind _returnvalue_21 (Math|Conversions|ToFloat(Integer) _returnvalue_16))
  (bind _returnvalue_22 (Math|Conversions|ToFloat(Integer) _returnvalue_15))
  (bind _returnvalue_23 (Math|Conversions|ToFloat(Integer) _returnvalue_17))
  (bind _returnvalue_24 (Math|Conversions|ToFloat(Integer) _returnvalue_18))
  (bind _returnvalue_25 (Math|Conversions|ToFloat(Integer) _returnvalue_19))
  (bind _returnvalue_26 (Math|Conversions|ToFloat(Integer) _returnvalue_20))
  (bind _s_pokefinalstats (Utilities|Struct|MakeS_PokeFinalStats _returnvalue_21 _returnvalue_21 _returnvalue_23 _returnvalue_23 _returnvalue_24 _returnvalue_24 _returnvalue_25 _returnvalue_25 _returnvalue_26 _returnvalue_26 _returnvalue_22 _returnvalue_22 _evasive _evasive _acuracy _acuracy))
  (Variables|Default|SetFinal%20Stats_0 _s_pokefinalstats)
  (return _s_pokefinalstats))
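; BP_make_players_use_lighting_channel is a box trigger volume that changes the lighting channels of player sprites inside it.
; When a BP_top_down_char begins overlapping, it saves that sprite's current channels, then applies the volume's three channel settings.
; On end overlap it restores the saved channels to the leaving character's sprite.
; Only one saved set exists per volume, so overlapping characters share it.
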(event `self.Box.OnComponentBeginOverlap`
  (params (OverlappedComponent :type "PrimitiveComponent Object Reference") (OtherActor :type "Actor Object Reference") (OtherComp :type "PrimitiveComponent Object Reference") (OtherBodyIndex :type Integer) (bFromSweep :type Boolean) (SweepResult :type "HitResult Structure (by ref)"))
  (bind _asbp_top_down_char (cast `/Game/charecter/BP_top_down_char` OtherActor))
  (bind _sprite (`PaperCharacter.Sprite` _asbp_top_down_char))
  (set `self.Lighting Channels` (`PrimitiveComponent.LightingChannels` _sprite))
  (`PrimitiveComponent.SetLightingChannels` _sprite (`self.lighting Channel 0`) (`self.lighting Channel 1`) (`self.lighting Channel 2`)))

(event `self.Box.OnComponentEndOverlap`
  (params (OverlappedComponent :type "PrimitiveComponent Object Reference") (OtherActor :type "Actor Object Reference") (OtherComp :type "PrimitiveComponent Object Reference") (OtherBodyIndex :type Integer))
  (bind (_bchannel0 _bchannel1 _bchannel2) (break `LightingChannels` (`self.Lighting Channels`)))
  (bind _asbp_top_down_char (cast `/Game/charecter/BP_top_down_char` OtherActor))
  (`PrimitiveComponent.SetLightingChannels` (`PaperCharacter.Sprite` _asbp_top_down_char) _bchannel0 _bchannel1 _bchannel2))

(fn `UserConstructionScript`)
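; BP_TallGrass is a tall grass world object that animates when something overlaps its box.
; An overlap counter tracks occupants, and the first entry swaps the static sprite for the Grass flipbook and plays it forward once.
; On exit, a two-pass loop decrements the count and, at zero, plays the flipbook backward faster, restores the sprite after a brief delay and resets the DoOnce.
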(event `self.Box.OnComponentBeginOverlap`
  (params (OverlappedComponent :type "PrimitiveComponent Object Reference") (OtherActor :type "Actor Object Reference") (OtherComp :type "PrimitiveComponent Object Reference") (OtherBodyIndex :type Integer) (bFromSweep :type Boolean) (SweepResult :type "HitResult Structure (by ref)"))
  (bind _grass (`self.Grass`))
  (`|ExecutionSequence`
    (:`then_0`
      (set `self.PPL Enter Count` (+ (`self.PPL Enter Count`) 1))
      (`SceneComponent.SetVisibility` (`self.Grass_Sprite1`) false false)
      (`SceneComponent.SetVisibility` (`self.Grass`) true false)
      (`/Engine/EditorBlueprintResources/StandardMacros.DoOnce` false :!label _label
        (:`Completed`
          (`PaperFlipbookComponent.SetPlayRate` _grass 1.0)
          (`PaperFlipbookComponent.PlayFromStart` _grass))))
    (:`then_1`
      (`/Engine/EditorBlueprintResources/StandardMacros.DoOnce` false
        (:`Completed`
          (`PaperFlipbookComponent.SetLooping` (`self.Grass`) false))))))

(event `self.Box.OnComponentEndOverlap`
  (params (OverlappedComponent :type "PrimitiveComponent Object Reference") (OtherActor :type "Actor Object Reference") (OtherComp :type "PrimitiveComponent Object Reference") (OtherBodyIndex :type Integer))
  (bind _grass (`self.Grass`))
  (for _ (range 2)
    (if (== (`self.PPL Enter Count`) 0)
      (`PaperFlipbookComponent.SetPlayRate` _grass 1.5)
      (`PaperFlipbookComponent.ReverseFromEnd` _grass)
      (`KismetSystemLibrary.Delay` 0.1)
      (`SceneComponent.SetVisibility` (`self.Grass_Sprite1`) true false)
      (`SceneComponent.SetVisibility` (`self.Grass`) false false)
      (goto _label :!via `Reset`)
      (else
        (set `self.PPL Enter Count` (- (`self.PPL Enter Count`) 1))))))

(fn `UserConstructionScript`)
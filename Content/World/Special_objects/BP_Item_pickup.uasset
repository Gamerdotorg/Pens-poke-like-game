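; BP_Item_pickup is a world pickup that adds an item to the top-down character's inventory.
; A box overlap by BP_top_down_char caches the character and enables player input on the pickup, and leaving disables it.
; Pressing E looks up ItemName in DT_Item_info and, for Misc Items only, increments that row struct's count in the ItemsInInventory map, then sets InvLOCK.
; The graph never destroys or hides the pickup.
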(event `self.Box.OnComponentBeginOverlap`
  (params (OverlappedComponent :type "PrimitiveComponent Object Reference") (OtherActor :type "Actor Object Reference") (OtherComp :type "PrimitiveComponent Object Reference") (OtherBodyIndex :type Integer) (bFromSweep :type Boolean) (SweepResult :type "HitResult Structure (by ref)"))
  (bind _asbp_top_down_char (cast `/Game/charecter/BP_top_down_char` OtherActor))
  (set `self.As BP Top Down Char` _asbp_top_down_char)
  (`self.EnableInput` (`GameplayStatics.GetPlayerController` 0)))

(event `self.Box.OnComponentEndOverlap`
  (params (OverlappedComponent :type "PrimitiveComponent Object Reference") (OtherActor :type "Actor Object Reference") (OtherComp :type "PrimitiveComponent Object Reference") (OtherBodyIndex :type Integer))
  (cast `/Game/charecter/BP_top_down_char` OtherActor)
  (`self.DisableInput` (`GameplayStatics.GetPlayerController` 0)))

(event `Key|E`
  (params (Key :type "Key Structure"))
  (bind _as_bp_top_down_char (`self.As BP Top Down Char`))
  (bind _itemsininventory (`/Game/charecter/BP_top_down_char.ItemsInInventory` (`self.As BP Top Down Char`)))
  (:`Pressed`
    (bind _returnvalue (`|GetDataTableRow` "/Game/Items/Items_info/DT_Item_info.DT_Item_info" (`self.Item Name`))
      (:`then`
        (switch `/Game/Items/Items_info/E_Item_Types` (`.ItemType_5_AC9E847F4E17124B4E94F6876F408013` (break `/Game/Items/Items_info/S_Item_info` _returnvalue))
          (:`NewEnumerator9`
            (if (`BlueprintMapLibrary.Map_Contains` _itemsininventory _returnvalue)
              (`BlueprintMapLibrary.Map_Add` (`/Game/charecter/BP_top_down_char.ItemsInInventory` _as_bp_top_down_char) _returnvalue (+ (`BlueprintMapLibrary.Map_Find` _itemsininventory _returnvalue) 1))
              (else
                (`BlueprintMapLibrary.Map_Add` (`/Game/charecter/BP_top_down_char.ItemsInInventory` (`self.As BP Top Down Char`)) _returnvalue 1)))
            (set `/Game/charecter/BP_top_down_char.?Inv LOCK` true _as_bp_top_down_char)))))))

(fn `UserConstructionScript`)
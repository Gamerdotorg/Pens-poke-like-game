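; BP_Vanashing_Button is a badge-gated button that makes an assigned world object vanish.
; Box overlap by the local top-down character enables interact input, and leaving calls DisableInput.
; On interact, holding the required gym badge hides the object, swaps the sprite, recolours the light and disables the Blocking collision.
; It also passes Blocking to the character's VanashingButton; a separate runonserver event, uncalled here, makes Blocking ignore the player pawn.
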(event `self.ReceiveBeginPlay`
  (`self.SetActorEnableCollision` (`self.Object to Vanish`) false))

(event `self.Box.OnComponentBeginOverlap`
  (params (OverlappedComponent :type "PrimitiveComponent Object Reference") (OtherActor :type "Actor Object Reference") (OtherComp :type "PrimitiveComponent Object Reference") (OtherBodyIndex :type Integer) (bFromSweep :type Boolean) (SweepResult :type "HitResult Structure (by ref)"))
  (bind _asbp_top_down_char (cast `/Game/charecter/BP_top_down_char` OtherActor))
  (if (== _asbp_top_down_char (`GameplayStatics.GetPlayerCharacter` 0))
    (`self.EnableInput` (`GameplayStatics.GetPlayerController` 0))))

(event `self.Box.OnComponentEndOverlap`
  (params (OverlappedComponent :type "PrimitiveComponent Object Reference") (OtherActor :type "Actor Object Reference") (OtherComp :type "PrimitiveComponent Object Reference") (OtherBodyIndex :type Integer))
  (bind _asbp_top_down_char (cast `/Game/charecter/BP_top_down_char` OtherActor))
  (if (== _asbp_top_down_char (`GameplayStatics.GetPlayerCharacter` 0))
    (`self.DisableInput` (`GameplayStatics.GetPlayerController` 0) null)))

(event `EnhancedInput|/Game/charecter/input/IA_Interact`
  (params (ActionValue :type Boolean) (ElapsedSeconds :type "Float (double-precision)") (TriggeredSeconds :type "Float (double-precision)") (InputAction :type "InputAction Object Reference" :default "/Game/charecter/input/IA_Interact.IA_Interact"))
  (bind _object_to_vanish (`self.Object to Vanish`))
  (:`Started`
    (bind _asbp_top_down_char (cast `/Game/charecter/BP_top_down_char` (`GameplayStatics.GetPlayerCharacter` 0)))
    (if (`KismetArrayLibrary.Array_Contains` (`/Game/charecter/BP_top_down_char.Gym Badges` _asbp_top_down_char) (`self.Required Badge`))
      (`self.SetActorHiddenInGame` _object_to_vanish true)
      (`self.SetActorEnableCollision` _object_to_vanish false)
      (`PaperSpriteComponent.SetSprite` (`self.PaperSprite`) "/Game/World/Special_objects/Vanashing_Wall_Button/Button_Sprite_1.Button_Sprite_1")
      (`/Game/charecter/BP_top_down_char.Vanashing Button` _asbp_top_down_char (`self.Blocking`))
      (`PrimitiveComponent.SetCollisionEnabled` (`self.Blocking`) "NoCollision")
      (`LightComponent.SetLightColor` (`self.RectLight`) (make `LinearColor` 0.0 255.0 0.0 1.0) true))))

(event `run on server`
  (`PrimitiveComponent.IgnoreActorWhenMoving` (`self.Blocking`) (`GameplayStatics.GetPlayerPawn` 0) true))

(fn `UserConstructionScript`)
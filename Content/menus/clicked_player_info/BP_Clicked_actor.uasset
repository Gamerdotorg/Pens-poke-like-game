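; BP_Clicked_actor is a short-lived actor for the clicked-player info menu, tied to a ChallangedActor reference.
; On BeginPlay it destroys every other instance of its class, so the newest one replaces the rest.
; Each Tick it destroys itself once the challenged actor is no longer within a fixed short distance of its location.
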(event `self.ReceiveBeginPlay`
  (bind _outactors (`GameplayStatics.GetAllActorsOfClass` "BP_Clicked_actor_C"))
  (for _array_element _outactors
    (if (not (== _array_element self))
      (`self.K2_DestroyActor` _array_element))))

(event `self.ReceiveTick`
  (params (DeltaSeconds :type "Float (single-precision)"))
  (if (not (< (`KismetMathLibrary.Vector_Distance` (`self.K2_GetActorLocation` (`self.Challanged Actor`)) (`self.K2_GetActorLocation`)) 200.0))
    (`self.K2_DestroyActor`)))

(fn `NewFunction`)

(fn `UserConstructionScript`)
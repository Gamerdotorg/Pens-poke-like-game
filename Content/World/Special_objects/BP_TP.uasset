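; BP_TP is a teleporter that moves the top-down character to a linked destination when it overlaps the box.
; On BeginPlay it sets the landing point 64 units from CarpetRef, offset along that reference's DirectionTP so the player arrives beside it.
; Carpet-type teleporters also spawn a BP_Carpet at their own transform, passing in their direction.
; The WASD key-check function is an unfinished stub with no actions.
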(event `self.ReceiveBeginPlay`
  (bind _returnvalue (`self.K2_GetActorLocation` (`self.Carpet ref`)))
  (switch `/Game/World/Special_objects/TP/Carpet/E_Directional_Tp` (`/Game/World/Special_objects/BP_TP.Direction TP` (`self.Carpet ref`))
    (:`NewEnumerator0`
      (set `self.Location to TP to` (- _returnvalue (0.0 64.0 0.0))))
    (:`NewEnumerator1`
      (set `self.Location to TP to` (- _returnvalue (0.0 -64.0 0.0))))
    (:`NewEnumerator2`
      (set `self.Location to TP to` (- _returnvalue (64.0 0.0 0.0))))
    (:`NewEnumerator3`
      (set `self.Location to TP to` (- _returnvalue (-64.0 0.0 0.0)))))
  (switch `/Game/World/Special_objects/TP/E_TP_Types` (`self.Type`)
    (:`NewEnumerator1`
      (`|SpawnActorFromClass` "/Game/World/Special_objects/TP/BP_Carpet.BP_Carpet_C" (`self.GetTransform` self) "Undefined" "MultiplyWithRoot" null (`self.Direction TP`) null))))

(event `self.Box.OnComponentBeginOverlap`
  (params (OverlappedComponent :type "PrimitiveComponent Object Reference") (OtherActor :type "Actor Object Reference") (OtherComp :type "PrimitiveComponent Object Reference") (OtherBodyIndex :type Integer) (bFromSweep :type Boolean) (SweepResult :type "HitResult Structure (by ref)"))
  (bind _asbp_top_down_char (cast `/Game/charecter/BP_top_down_char` OtherActor))
  (`self.K2_SetActorLocation` _asbp_top_down_char (`self.Location to TP to`) false true))

(fn `UserConstructionScript`)

(fn `What Key Was just pressed`
  (`|ExecutionSequence`
    (:`then_0`
      (if (`PlayerController.WasInputKeyJustPressed` (`GameplayStatics.GetPlayerController` 0) "W")
        _))
    (:`then_1`
      (if (`PlayerController.WasInputKeyJustPressed` (`GameplayStatics.GetPlayerController` 0) "S")
        _))
    (:`then_2`
      (if (`PlayerController.WasInputKeyJustPressed` (`GameplayStatics.GetPlayerController` 0) "A")
        _))
    (:`then_3`
      (if (`PlayerController.WasInputKeyJustPressed` (`GameplayStatics.GetPlayerController` 0) "D")
        _))))
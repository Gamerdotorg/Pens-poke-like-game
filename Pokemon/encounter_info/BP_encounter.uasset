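; Wild Pokémon encounter zone that starts a battle while the player moves inside its box.
; A looping timer rolls each second, with odds rising after every failed roll.
; A success picks a species by weighted random from PossiblePokemon, then rolls shininess, gender, route-based level, IVs, stats and up to four level-up moves from data tables.
; The resulting EncounterPokemon goes to BP_top_down_char as the enemy team through SpBattleStart.
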(event OnComponentBeginOverlap(Box)
  (params (OverlappedComponent :type Primitive%20Component%20Object%20Reference) (OtherActor :type Actor%20Object%20Reference) (OtherComp :type Primitive%20Component%20Object%20Reference) (OtherBodyIndex :type Integer) (bFromSweep :type Boolean) (SweepResult :type Hit%20Result%20Structure%20%28by%20ref%29))
  (bind _asbp_top_down_char (Utilities|Casting|CastToBP_top_down_char OtherActor))
  (if (Utilities|IsValid (Components|GetOwner _asbp_top_down_char))
    (bind _output_get (Variables|Default|SetPlayer%20Ref _asbp_top_down_char))
    (Variables|/Game/charecter/BP_top_down_char.BP_top_down_char_C|SetEncounter%20Box%20Ref _output_get self)
    (bind _returnvalue (Utilities|Time|SetTimerbyEvent (delegate Custom|Roll%20For%20Encounter) 1.0 true))
    (Variables|Default|SetSpawn%20Timer _returnvalue)))

(event OnComponentEndOverlap(Box)
  (params (OverlappedComponent :type Primitive%20Component%20Object%20Reference) (OtherActor :type Actor%20Object%20Reference) (OtherComp :type Primitive%20Component%20Object%20Reference) (OtherBodyIndex :type Integer))
  (Utilities|Casting|CastToBP_top_down_char OtherActor)
  (Utilities|Time|ClearandInvalidateTimerbyHandle (Variables|Default|GetSpawn%20Timer)))

(event Custom|Roll%20For%20Encounter
  (if (> (Math|Vector|VectorLengthXY (Variables|/Script/Engine.MovementComponent|GetVelocity (Variables|/Script/Engine.Character|GetCharacterMovement (Variables|Default|GetPlayer%20Ref)))) 0.1)
    (if (Math|Random|RandomBoolwithWeight (+ (Math|Float|MakeLiteralFloat 0.1) (* (Variables|Default|GetTimes%20Roll%20Failed) 0.05)))
      (Variables|Default|SetTimes%20Roll%20Failed 0)
      (CallFunction|SetEncounter)
      (else
        (Math|Integer|IncrementInt (Variables|Default|GetTimes%20Roll%20Failed))))))

(event Custom|Set%20encounter
  (Utilities|Array|Clear (Variables|Default|GetEnemy%20Team))
  (if (== (Math|Random|RandomIntegerinRange 1 8000) 1)
    (Variables|Default|SetisShiny? true)
    (else
      (Variables|Default|SetisShiny? false)))
  (if (>= (Math|Random|RandomIntegerinRange 1 100) 51)
    (Variables|Default|SetGender "NewEnumerator1")
    (else
      (Variables|Default|SetGender "NewEnumerator2")))
  (bind _pokemon_name (CallFunction|ChooseEncounter))
  (bind _returnvalue (Utilities|GetDataTableRow "/Game/Pokemon/info/DT_Pokemon_basic_info.DT_Pokemon_basic_info" _pokemon_name)
    (:then
      (CallFunction|SetEncounterInfo _returnvalue)
      (CallFunction|RollIV)
      (CallFunction|RollFinalStats _pokemon_name)
      (CallFunction|RollMoveSlots)
      (Utilities|Array|Add (Variables|Default|GetEnemy%20Team) (Variables|Default|Getencounter%20pokemon))
      (bind _asbp_top_down_char (Utilities|Casting|CastToBP_top_down_char (Game|GetPlayerCharacter 0)))
      (Default|SpBattleStart _asbp_top_down_char (Variables|Default|GetEnemy%20Team) true))
    (:RowNotFound
      (Development|PrintString "no pokemon found"))))

(fn ConstructionScript)

(fn ChooseEncounter
  (bind _possible_pokemon (Variables|Default|GetPossible%20Pokemon))
  (bind _pokemonname (Utilities|Struct|BreakS_Possible_encounters _possible_pokemon))
  (LocalVariables|Setsum%20of%20array 0.0)
  (bind _values (Utilities|Map|Values (Utilities|Struct|BreakS_Possible_encounters (Variables|Default|GetPossible%20Pokemon))))
  (for _array_element _values
    (LocalVariables|Setsum%20of%20array (+ _array_element (LocalVariables|Getsum%20of%20array))))
  (LocalVariables|SetRoll (Math|Random|RandomFloatinRange 0.0 (LocalVariables|Getsum%20of%20array)))
  (bind _keys (Utilities|Map|Keys _pokemonname))
  (bind _array_element_2 (Utilities|Array|ForEachLoopwithBreak _keys :!label _label)
    (:LoopBody
      (if (>= (.Value (Utilities|Map|Find _pokemonname _array_element_2)) (LocalVariables|GetRoll))
        (bind _output_get (LocalVariables|SetChosen%20Encounter _array_element_2))
        (Development|PrintString (Utilities|String|ToString(Name) _output_get))
        (goto _label Break)
        (else
          (LocalVariables|SetRoll (- (LocalVariables|GetRoll) (.Value (Utilities|Map|Find _pokemonname _array_element_2)))))))
    (:Completed
      (return (LocalVariables|GetChosen%20Encounter)))))

(fn SetEncounterInfo
  (params (Poke%20basic%20info :type S%20Poke%20Basic%20Information%20Structure))
  (bind _returnvalue (Utilities|GetDataTableRow (Variables|Default|GetRoute%20Info) (Utilities|Struct|BreakS_PokeBasicInformation Poke%20basic%20info))
    (:then
      (bind _structout (Utilities|Struct|SetmembersinS_PokePartyInfo (Variables|Default|Getencounter%20pokemon) (.PokemonName (Utilities|Struct|BreakS_Encounter _returnvalue)) (Utilities|String|ToString(Name) (.PokemonName (Utilities|Struct|BreakS_Encounter _returnvalue))) (Math|Random|RandomIntegerinRange (.MinLevel (Utilities|Struct|BreakS_Encounter _returnvalue)) (.MaxLevel (Utilities|Struct|BreakS_Encounter _returnvalue))) (Variables|Default|GetisShiny?) (Variables|Default|GetGender)))
      (Variables|Default|Setencounter%20pokemon _structout)
      (return))))

(fn RollIV
  (bind _structout (Utilities|Struct|SetmembersinS_PokePartyInfo (Variables|Default|Getencounter%20pokemon) (Utilities|Struct|MakeS_PokeIV (Math|Random|RandomIntegerinRange 0 31) (Math|Random|RandomIntegerinRange 0 31) (Math|Random|RandomIntegerinRange 0 31) (Math|Random|RandomIntegerinRange 0 31) (Math|Random|RandomIntegerinRange 0 31) (Math|Random|RandomIntegerinRange 0 31))))
  (Variables|Default|Setencounter%20pokemon _structout)
  (return))

(fn RollFinalStats
  (params (Pokemon%20Name :type Name))
  (bind _returnvalue (Utilities|GetDataTableRow "/Game/Pokemon/info/DT_Pokemon_basic_info.DT_Pokemon_basic_info" Pokemon%20Name)
    (:then
      (bind _structout (Utilities|Struct|SetmembersinS_PokePartyInfo (Variables|Default|Getencounter%20pokemon) (/ (* (* (* (.CurrentLevel (Utilities|Struct|BreakS_PokePartyInfo (Variables|Default|Getencounter%20pokemon))) 4) (.CurrentLevel (Utilities|Struct|BreakS_PokePartyInfo (Variables|Default|Getencounter%20pokemon)))) (.CurrentLevel (Utilities|Struct|BreakS_PokePartyInfo (Variables|Default|Getencounter%20pokemon)))) 5) (.BaseStatInformation (Utilities|Struct|BreakS_PokeBasicInformation _returnvalue)) (Utilities|Struct|MakeS_PokeFinalStats (Math|Conversions|ToFloat(Integer) (Math|Float|Round (|((((((HPBS*2)+HP)+CL)/100)+CL)+10) (.HP (Utilities|Struct|BreakS_PokeBaseStats (.BaseStatInformation (Utilities|Struct|BreakS_PokeBasicInformation _returnvalue)))) (.HP (Utilities|Struct|BreakS_PokeIV (.PokeIvs (Utilities|Struct|BreakS_PokePartyInfo (Variables|Default|Getencounter%20pokemon))))) (.CurrentLevel (Utilities|Struct|BreakS_PokePartyInfo (Variables|Default|Getencounter%20pokemon)))))) (Math|Conversions|ToFloat(Integer) (Math|Float|Round (|((((((HPBS*2)+HP)+CL)/100)+CL)+10) (.HP (Utilities|Struct|BreakS_PokeBaseStats (.BaseStatInformation (Utilities|Struct|BreakS_PokeBasicInformation _returnvalue)))) (.HP (Utilities|Struct|BreakS_PokeIV (.PokeIvs (Utilities|Struct|BreakS_PokePartyInfo (Variables|Default|Getencounter%20pokemon))))) (.CurrentLevel (Utilities|Struct|BreakS_PokePartyInfo (Variables|Default|Getencounter%20pokemon)))))) (Math|Conversions|ToFloat(Integer) (Math|Float|Round (|((((((StatBS*2)+IV)*CL)/100)+CL)+5) (.Attack (Utilities|Struct|BreakS_PokeBaseStats (.BaseStatInformation (Utilities|Struct|BreakS_PokeBasicInformation _returnvalue)))) (.ATTK (Utilities|Struct|BreakS_PokeIV (.PokeIvs (Utilities|Struct|BreakS_PokePartyInfo (Variables|Default|Getencounter%20pokemon))))) (.CurrentLevel (Utilities|Struct|BreakS_PokePartyInfo (Variables|Default|Getencounter%20pokemon)))))) (Math|Conversions|ToFloat(Integer) (Math|Float|Round (|((((((StatBS*2)+IV)*CL)/100)+CL)+5) (.Attack (Utilities|Struct|BreakS_PokeBaseStats (.BaseStatInformation (Utilities|Struct|BreakS_PokeBasicInformation _returnvalue)))) (.ATTK (Utilities|Struct|BreakS_PokeIV (.PokeIvs (Utilities|Struct|BreakS_PokePartyInfo (Variables|Default|Getencounter%20pokemon))))) (.CurrentLevel (Utilities|Struct|BreakS_PokePartyInfo (Variables|Default|Getencounter%20pokemon)))))) (Math|Conversions|ToFloat(Integer) (Math|Float|Round (|((((((StatBS*2)+IV)*CL)/100)+CL)+5) (.Defence (Utilities|Struct|BreakS_PokeBaseStats (.BaseStatInformation (Utilities|Struct|BreakS_PokeBasicInformation _returnvalue)))) (.DEF (Utilities|Struct|BreakS_PokeIV (.PokeIvs (Utilities|Struct|BreakS_PokePartyInfo (Variables|Default|Getencounter%20pokemon))))) (.CurrentLevel (Utilities|Struct|BreakS_PokePartyInfo (Variables|Default|Getencounter%20pokemon)))))) (Math|Conversions|ToFloat(Integer) (Math|Float|Round (|((((((StatBS*2)+IV)*CL)/100)+CL)+5) (.Defence (Utilities|Struct|BreakS_PokeBaseStats (.BaseStatInformation (Utilities|Struct|BreakS_PokeBasicInformation _returnvalue)))) (.DEF (Utilities|Struct|BreakS_PokeIV (.PokeIvs (Utilities|Struct|BreakS_PokePartyInfo (Variables|Default|Getencounter%20pokemon))))) (.CurrentLevel (Utilities|Struct|BreakS_PokePartyInfo (Variables|Default|Getencounter%20pokemon)))))) (Math|Conversions|ToFloat(Integer) (Math|Float|Round (|((((((StatBS*2)+IV)*CL)/100)+CL)+5) (.SPAttack (Utilities|Struct|BreakS_PokeBaseStats (.BaseStatInformation (Utilities|Struct|BreakS_PokeBasicInformation _returnvalue)))) (.SP_ATTK (Utilities|Struct|BreakS_PokeIV (.PokeIvs (Utilities|Struct|BreakS_PokePartyInfo (Variables|Default|Getencounter%20pokemon))))) (.CurrentLevel (Utilities|Struct|BreakS_PokePartyInfo (Variables|Default|Getencounter%20pokemon)))))) (Math|Conversions|ToFloat(Integer) (Math|Float|Round (|((((((StatBS*2)+IV)*CL)/100)+CL)+5) (.SPAttack (Utilities|Struct|BreakS_PokeBaseStats (.BaseStatInformation (Utilities|Struct|BreakS_PokeBasicInformation _returnvalue)))) (.SP_ATTK (Utilities|Struct|BreakS_PokeIV (.PokeIvs (Utilities|Struct|BreakS_PokePartyInfo (Variables|Default|Getencounter%20pokemon))))) (.CurrentLevel (Utilities|Struct|BreakS_PokePartyInfo (Variables|Default|Getencounter%20pokemon)))))) (Math|Conversions|ToFloat(Integer) (Math|Float|Round (|((((((StatBS*2)+IV)*CL)/100)+CL)+5) (.SPDefence (Utilities|Struct|BreakS_PokeBaseStats (.BaseStatInformation (Utilities|Struct|BreakS_PokeBasicInformation _returnvalue)))) (.SP_DEF (Utilities|Struct|BreakS_PokeIV (.PokeIvs (Utilities|Struct|BreakS_PokePartyInfo (Variables|Default|Getencounter%20pokemon))))) (.CurrentLevel (Utilities|Struct|BreakS_PokePartyInfo (Variables|Default|Getencounter%20pokemon)))))) (Math|Conversions|ToFloat(Integer) (Math|Float|Round (|((((((StatBS*2)+IV)*CL)/100)+CL)+5) (.SPDefence (Utilities|Struct|BreakS_PokeBaseStats (.BaseStatInformation (Utilities|Struct|BreakS_PokeBasicInformation _returnvalue)))) (.SP_DEF (Utilities|Struct|BreakS_PokeIV (.PokeIvs (Utilities|Struct|BreakS_PokePartyInfo (Variables|Default|Getencounter%20pokemon))))) (.CurrentLevel (Utilities|Struct|BreakS_PokePartyInfo (Variables|Default|Getencounter%20pokemon)))))) (Math|Conversions|ToFloat(Integer) (Math|Float|Round (|((((((StatBS*2)+IV)*CL)/100)+CL)+5) (.Speed (Utilities|Struct|BreakS_PokeBaseStats (.BaseStatInformation (Utilities|Struct|BreakS_PokeBasicInformation _returnvalue)))) (.SPEED (Utilities|Struct|BreakS_PokeIV (.PokeIvs (Utilities|Struct|BreakS_PokePartyInfo (Variables|Default|Getencounter%20pokemon))))) (.CurrentLevel (Utilities|Struct|BreakS_PokePartyInfo (Variables|Default|Getencounter%20pokemon)))))) (Math|Conversions|ToFloat(Integer) (Math|Float|Round (|((((((StatBS*2)+IV)*CL)/100)+CL)+5) (.Speed (Utilities|Struct|BreakS_PokeBaseStats (.BaseStatInformation (Utilities|Struct|BreakS_PokeBasicInformation _returnvalue)))) (.SPEED (Utilities|Struct|BreakS_PokeIV (.PokeIvs (Utilities|Struct|BreakS_PokePartyInfo (Variables|Default|Getencounter%20pokemon))))) (.CurrentLevel (Utilities|Struct|BreakS_PokePartyInfo (Variables|Default|Getencounter%20pokemon)))))) (.Evasive (Utilities|Struct|BreakS_PokeBaseStats (.BaseStatInformation (Utilities|Struct|BreakS_PokeBasicInformation _returnvalue)))) (.Evasive (Utilities|Struct|BreakS_PokeBaseStats (.BaseStatInformation (Utilities|Struct|BreakS_PokeBasicInformation _returnvalue)))) (.Acuracy (Utilities|Struct|BreakS_PokeBaseStats (.BaseStatInformation (Utilities|Struct|BreakS_PokeBasicInformation _returnvalue)))) (.Acuracy (Utilities|Struct|BreakS_PokeBaseStats (.BaseStatInformation (Utilities|Struct|BreakS_PokeBasicInformation _returnvalue)))))))
      (Variables|Default|Setencounter%20pokemon _structout))))

(fn RollMoveSlots
  (bind _possible_moves (Variables|Default|Getpossible%20moves))
  (bind _returnvalue (Utilities|Array|LastIndex _possible_moves))
  (bind _outrownames (DataTable|GetDataTableRowNames "/Game/Pokemon/info/DT_pokemon_move.DT_pokemon_move"))
  (for _array_element _outrownames
    (if (.ReturnValue (Utilities|Map|Find (Utilities|Struct|BreakS_PokeBaseStats (.Basestats (Utilities|Struct|BreakS_PokePartyInfo (Variables|Default|Getencounter%20pokemon)))) _array_element))
      (if (<= (.Value (Utilities|Map|Find (Utilities|Struct|BreakS_PokeBaseStats (.Basestats (Utilities|Struct|BreakS_PokePartyInfo (Variables|Default|Getencounter%20pokemon)))) _array_element)) (.CurrentLevel (Utilities|Struct|BreakS_PokePartyInfo (Variables|Default|Getencounter%20pokemon))))
        (Utilities|Array|Add (Variables|Default|Getpossible%20moves) (.Value (Utilities|Map|Find (Utilities|Struct|BreakS_PokeBaseStats (.Basestats (Utilities|Struct|BreakS_PokePartyInfo (Variables|Default|Getencounter%20pokemon)))) _array_element))))))
  (bind _keys (Utilities|Map|Keys (Utilities|Struct|BreakS_PokeBaseStats (.Basestats (Utilities|Struct|BreakS_PokePartyInfo (Variables|Default|Getencounter%20pokemon))))))
  (for _index (range 0 3)
    (if (> (Utilities|Array|Length _possible_moves) 0)
      (bind _returnvalue_2 (Utilities|GetDataTableRow "/Game/Pokemon/info/DT_pokemon_move.DT_pokemon_move" (Utilities|Array|Get(acopy) _keys _returnvalue))
        (:then
          (Utilities|Array|AddUnique (Variables|Default|Getmoves) (Utilities|Struct|BreakS_Move _returnvalue_2))
          (Utilities|Array|RemoveIndex (Variables|Default|Getpossible%20moves) _returnvalue)))))
  (bind _structout (Utilities|Struct|SetmembersinS_PokePartyInfo (Variables|Default|Getencounter%20pokemon) (Variables|Default|Getmoves)))
  (Variables|Default|Setencounter%20pokemon _structout)
  (return))
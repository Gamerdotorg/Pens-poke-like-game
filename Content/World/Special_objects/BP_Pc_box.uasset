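; BP_Pc_box is an interactable world object that opens the PokeBox widget for the player.
; Its Box overlap enables input on the actor while the player's BP_top_down_char is inside and disables it when the player leaves.
; Pressing IA_Interact creates a new W_PokeBox widget and adds it to the viewport, with no check for one already open.
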(event `self.Box.OnComponentBeginOverlap`
  (params (OverlappedComponent :type "PrimitiveComponent Object Reference") (OtherActor :type "Actor Object Reference") (OtherComp :type "PrimitiveComponent Object Reference") (OtherBodyIndex :type Integer) (bFromSweep :type Boolean) (SweepResult :type "HitResult Structure (by ref)"))
  (bind _asbp_top_down_char (cast `/Game/charecter/BP_top_down_char` OtherActor))
  (if (== _asbp_top_down_char (`GameplayStatics.GetPlayerCharacter` 0))
    (`self.EnableInput` (`GameplayStatics.GetPlayerController` 0))))

(event `self.Box.OnComponentEndOverlap`
  (params (OverlappedComponent :type "PrimitiveComponent Object Reference") (OtherActor :type "Actor Object Reference") (OtherComp :type "PrimitiveComponent Object Reference") (OtherBodyIndex :type Integer))
  (bind _asbp_top_down_char (cast `/Game/charecter/BP_top_down_char` OtherActor))
  (if (== _asbp_top_down_char (`GameplayStatics.GetPlayerCharacter` 0))
    (`self.DisableInput` (`GameplayStatics.GetPlayerController` 0))))

(event `EnhancedInput|/Game/charecter/input/IA_Interact`
  (params (ActionValue :type Boolean) (ElapsedSeconds :type "Float (double-precision)") (TriggeredSeconds :type "Float (double-precision)") (InputAction :type "InputAction Object Reference" :default "/Game/charecter/input/IA_Interact.IA_Interact"))
  (:`Started`
    (cast `/Game/charecter/BP_top_down_char` (`GameplayStatics.GetPlayerCharacter` 0))
    (bind _returnvalue (`|CreateWidget` "/Game/menus/PokeBox/W_PokeBox.W_PokeBox_C"))
    (`UserWidget.AddToViewport` _returnvalue 0)))

(fn `UserConstructionScript`)
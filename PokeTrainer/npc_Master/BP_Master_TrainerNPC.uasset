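; Master trainer NPC that starts a battle with its team when an unbeaten trainer's sight box overlaps the player.
; BeginPlay enables the hitbox for LookingDirection, though only the south box's overlap is wired to start battles.
; It also fills TrainerTeam from GivenPokemon, using data-table base stats and random-IV stat formulas.
; FinalStats runs before each entry's level and base stats are set; interaction logic is unfinished.
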(event OnComponentBeginOverlap(InteractHitBox)
  (params (OverlappedComponent :type Primitive%20Component%20Object%20Reference) (OtherActor :type Actor%20Object%20Reference) (OtherComp :type Primitive%20Component%20Object%20Reference) (OtherBodyIndex :type Integer) (bFromSweep :type Boolean) (SweepResult :type Hit%20Result%20Structure%20%28by%20ref%29)))

(event OnComponentBeginOverlap(EastHitBox)
  (params (OverlappedComponent :type Primitive%20Component%20Object%20Reference) (OtherActor :type Actor%20Object%20Reference) (OtherComp :type Primitive%20Component%20Object%20Reference) (OtherBodyIndex :type Integer) (bFromSweep :type Boolean) (SweepResult :type Hit%20Result%20Structure%20%28by%20ref%29)))

(event OnComponentBeginOverlap(SouthHitBox)
  (params (OverlappedComponent :type Primitive%20Component%20Object%20Reference) (OtherActor :type Actor%20Object%20Reference) (OtherComp :type Primitive%20Component%20Object%20Reference) (OtherBodyIndex :type Integer) (bFromSweep :type Boolean) (SweepResult :type Hit%20Result%20Structure%20%28by%20ref%29))
  (CallFunction|OverlapFunc OtherActor))

(event OnComponentBeginOverlap(NorthHitBox)
  (params (OverlappedComponent :type Primitive%20Component%20Object%20Reference) (OtherActor :type Actor%20Object%20Reference) (OtherComp :type Primitive%20Component%20Object%20Reference) (OtherBodyIndex :type Integer) (bFromSweep :type Boolean) (SweepResult :type Hit%20Result%20Structure%20%28by%20ref%29)))

(event OnComponentBeginOverlap(WestHitBox)
  (params (OverlappedComponent :type Primitive%20Component%20Object%20Reference) (OtherActor :type Actor%20Object%20Reference) (OtherComp :type Primitive%20Component%20Object%20Reference) (OtherBodyIndex :type Integer) (bFromSweep :type Boolean) (SweepResult :type Hit%20Result%20Structure%20%28by%20ref%29)))

(event OnComponentEndOverlap(InteractHitBox)
  (params (OverlappedComponent :type Primitive%20Component%20Object%20Reference) (OtherActor :type Actor%20Object%20Reference) (OtherComp :type Primitive%20Component%20Object%20Reference) (OtherBodyIndex :type Integer)))

(event Input|EnhancedActionEvents|EnhancedInputActionIA_Interact
  (params (ActionValue :type Boolean) (ElapsedSeconds :type Float%20%28double-precision%29) (TriggeredSeconds :type Float%20%28double-precision%29) (InputAction :type Input%20Action%20Object%20Reference :default "/Game/charecter/input/IA_Interact.IA_Interact")))

(event EventBeginPlay
  (CallFunction|DirectionLookin)
  (CallFunction|GivePokemonj))

(fn ConstructionScript)

(fn OverlapFunc
  (params (Other%20Actor :type Actor%20Object%20Reference) (This%20Hit%20Box :type Box%20Component%20Object%20Reference))
  (if (not (Variables|Default|Get?Beaten))
    (bind _asbp_top_down_char (Utilities|Casting|CastToBP_top_down_char Other%20Actor))
    (if (Utilities|IsValid (Components|GetOwner _asbp_top_down_char))
      (bind _output_get (Variables|Default|SetPlayer%20ref _asbp_top_down_char))
      (Default|SpBattleStart _output_get (Variables|GivePokemon|GetTrainer%20Team) false)
      (return))))

(fn GivePokemonj
  (for (_array_element _array_index) (Variables|Default|GetGiven%20Pokemon)
    (CallFunction|FinalStats)
    (Variables|GivePokemon|SetLevel (.Level (Utilities|Struct|BreakS_Trainer_Party_info _array_element)))
    (bind _returnvalue (Utilities|GetDataTableRow "/Game/Pokemon/info/DT_Pokemon_basic_info.DT_Pokemon_basic_info" (.PokemonName (Utilities|Struct|BreakS_Trainer_Party_info _array_element)))
      (:then
        (Variables|GivePokemon|SetBase%20Stats (Utilities|Struct|MakeS_PokeBaseStats (.HP (Utilities|Struct|BreakS_PokeBaseStats (Utilities|Struct|BreakS_PokeBasicInformation _returnvalue))) (.Attack (Utilities|Struct|BreakS_PokeBaseStats (Utilities|Struct|BreakS_PokeBasicInformation _returnvalue))) (.Defence (Utilities|Struct|BreakS_PokeBaseStats (Utilities|Struct|BreakS_PokeBasicInformation _returnvalue))) (.SPAttack (Utilities|Struct|BreakS_PokeBaseStats (Utilities|Struct|BreakS_PokeBasicInformation _returnvalue))) (.SPDefence (Utilities|Struct|BreakS_PokeBaseStats (Utilities|Struct|BreakS_PokeBasicInformation _returnvalue))) (.Speed (Utilities|Struct|BreakS_PokeBaseStats (Utilities|Struct|BreakS_PokeBasicInformation _returnvalue))) (.Acuracy (Utilities|Struct|BreakS_PokeBaseStats (Utilities|Struct|BreakS_PokeBasicInformation _returnvalue))) (.Evasive (Utilities|Struct|BreakS_PokeBaseStats (Utilities|Struct|BreakS_PokeBasicInformation _returnvalue))) (.LevelUPMoveSet (Utilities|Struct|BreakS_PokeBaseStats (Utilities|Struct|BreakS_PokeBasicInformation _returnvalue))) (.TMMoves (Utilities|Struct|BreakS_PokeBaseStats (Utilities|Struct|BreakS_PokeBasicInformation _returnvalue)))))
        (Utilities|Array|SetArrayElem (Variables|GivePokemon|GetTrainer%20Team) _array_index (Utilities|Struct|MakeS_PokePartyInfo (.PokemonName (Utilities|Struct|BreakS_Trainer_Party_info _array_element)) (Utilities|String|ToString(Name) (.PokemonName (Utilities|Struct|BreakS_Trainer_Party_info _array_element))) "NewEnumerator0" "None" (.moves (Utilities|Struct|BreakS_Trainer_Party_info _array_element)) 0 1.0 1e+01 (Variables|GivePokemon|GetLevel) false "NewEnumerator0" 255 (Variables|GivePokemon|GetBase%20Stats) "(HP_12_7B44F36E4B5ABC0A420A06B178113116=0,ATTK_13_115EAC5A41856E4DC1B430A715F799F0=0,DEF_14_D56CDB354B1E19CE588FB982BD399DAC=0,SP_ATTK_15_DE5FA0BD475C036FC45A5883B981C2C6=0,SP_DEF_16_29222FA440814E2D2B06B79DBFECE523=0,SPEED_17_748E4BFA44002EE1611C41951707FEFA=0)" "(HP_12_7B44F36E4B5ABC0A420A06B178113116=0,ATTK_13_115EAC5A41856E4DC1B430A715F799F0=0,DEF_14_D56CDB354B1E19CE588FB982BD399DAC=0,SP_ATTK_15_DE5FA0BD475C036FC45A5883B981C2C6=0,SP_DEF_16_29222FA440814E2D2B06B79DBFECE523=0,SPEED_17_748E4BFA44002EE1611C41951707FEFA=0)" (Variables|GivePokemon|GetS%20Poke%20Final%20Stats)))))))

(fn FinalStats
  (bind _returnvalue (Math|Random|RandomIntegerinRange 0 31))
  (bind _returnvalue_2 (Math|Random|RandomIntegerinRange 0 31))
  (bind _returnvalue_3 (Math|Random|RandomIntegerinRange 0 31))
  (bind _returnvalue_4 (Math|Random|RandomIntegerinRange 0 31))
  (bind _returnvalue_5 (Math|Random|RandomIntegerinRange 0 31))
  (bind _returnvalue_6 (Math|Random|RandomIntegerinRange 0 31))
  (bind _base_stats (Variables|GivePokemon|GetBase%20Stats))
  (bind _level (Variables|GivePokemon|GetLevel))
  (bind (_hp _attack _defence _spattack _spdefence _speed _acuracy _evasive) (Utilities|Struct|BreakS_PokeBaseStats _base_stats))
  (bind _s_pokeiv (Utilities|Struct|MakeS_PokeIV _returnvalue_2 _returnvalue_3 _returnvalue_4 _returnvalue_5 _returnvalue_6 _returnvalue))
  (bind (_hp_2 _attk _def _sp_attk _sp_def _speed_2) (Utilities|Struct|BreakS_PokeIV _s_pokeiv))
  (bind _returnvalue_7 (|((((((HPBS*2)+HP)+CL)/100)+CL)+10) _hp _hp_2 _level))
  (bind _returnvalue_8 (|((((((StatBS*2)+IV)*CL)/100)+CL)+5) _speed _speed_2 _level))
  (bind _returnvalue_9 (|((((((StatBS*2)+IV)*CL)/100)+CL)+5) _attack _attk _level))
  (bind _returnvalue_10 (|((((((StatBS*2)+IV)*CL)/100)+CL)+5) _defence _def _level))
  (bind _returnvalue_11 (|((((((StatBS*2)+IV)*CL)/100)+CL)+5) _spattack _sp_attk _level))
  (bind _returnvalue_12 (|((((((StatBS*2)+IV)*CL)/100)+CL)+5) _spdefence _sp_def _level))
  (bind _returnvalue_13 (Math|Float|Round _returnvalue_8))
  (bind _returnvalue_14 (Math|Float|Round _returnvalue_7))
  (bind _returnvalue_15 (Math|Float|Round _returnvalue_9))
  (bind _returnvalue_16 (Math|Float|Round _returnvalue_10))
  (bind _returnvalue_17 (Math|Float|Round _returnvalue_11))
  (bind _returnvalue_18 (Math|Float|Round _returnvalue_12))
  (bind _returnvalue_19 (Math|Conversions|ToFloat(Integer) _returnvalue_14))
  (bind _returnvalue_20 (Math|Conversions|ToFloat(Integer) _returnvalue_13))
  (bind _returnvalue_21 (Math|Conversions|ToFloat(Integer) _returnvalue_15))
  (bind _returnvalue_22 (Math|Conversions|ToFloat(Integer) _returnvalue_16))
  (bind _returnvalue_23 (Math|Conversions|ToFloat(Integer) _returnvalue_17))
  (bind _returnvalue_24 (Math|Conversions|ToFloat(Integer) _returnvalue_18))
  (Variables|GivePokemon|SetS%20Poke%20Final%20Stats (Utilities|Struct|MakeS_PokeFinalStats _returnvalue_19 _returnvalue_19 _returnvalue_21 _returnvalue_21 _returnvalue_22 _returnvalue_22 _returnvalue_23 _returnvalue_23 _returnvalue_24 _returnvalue_24 _returnvalue_20 _returnvalue_20 _evasive _evasive _acuracy _acuracy))
  (return))

(fn DirectionLookin
  (switch Utilities|FlowControl|Switch|SwitchonE_Direction_NPC (Variables|Default|GetLooking%20direction)
    (:NewEnumerator4
      (Variables|Default|SetDirectionality "(X=0.000000,Y=-1.000000)")
      (Collision|SetCollisionEnabled (Variables|Default|GetEast%20Hit%20Box) "NoCollision"))
    (:NewEnumerator0
      (Variables|Default|SetDirectionality "(X=0.000000,Y=1.000000)")
      (Collision|SetCollisionEnabled (Variables|Default|GetNorth%20Hit%20Box) "QueryAndPhysics")
      (Collision|SetCollisionEnabled (Variables|Default|GetEast%20Hit%20Box) "NoCollision"))
    (:NewEnumerator1
      (Variables|Default|SetDirectionality "(X=1.000000,Y=0.000000)")
      (Collision|SetCollisionEnabled (Variables|Default|GetEast%20Hit%20Box) "QueryAndPhysics")
      (Collision|SetCollisionEnabled (Variables|Default|GetNorth%20Hit%20Box) "NoCollision"))
    (:NewEnumerator2
      (Variables|Default|SetDirectionality "(X=0.000000,Y=-1.000000)")
      (Collision|SetCollisionEnabled (Variables|Default|GetSouth%20Hit%20Box) "QueryAndPhysics")
      (Collision|SetCollisionEnabled (Variables|Default|GetEast%20Hit%20Box) "NoCollision"))
    (:NewEnumerator3
      (Variables|Default|SetDirectionality "(X=-1.000000,Y=0.000000)")
      (Collision|SetCollisionEnabled (Variables|Default|GetWest%20Hit%20Box) "QueryAndPhysics")
      (Collision|SetCollisionEnabled (Variables|Default|GetEast%20Hit%20Box) "NoCollision"))))

(fn InteractwithNpc
  (switch Utilities|FlowControl|Switch|SwitchonE_NPC_Types (Variables|Default|GetE_npc%20Type)))

(fn ?npcType
  (switch Utilities|FlowControl|Switch|SwitchonE_NPC_Types (Variables|Default|GetE_npc%20Type)))

(fn AddMapingContext)